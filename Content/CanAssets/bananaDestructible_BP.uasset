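; Banana destructible actor in CanAssets that animates a Destructible component falling and scaling when it spawns.
; On BeginPlay a timeline drives the component's relative location from its Fall track and relative scale from its ScaleAnim track, teleporting without sweep.
; An ApplyDamage call and a random can-label material pick in the construction script are left unconnected, so neither runs.
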(event EventBeginPlay
  (bind _destructible (Variables|Default|GetDestructible))
  (bind (_direction _fall _scaleanim) (Timeline|Timeline_0 PlayFromStart)
    (:Update
      (Transformation|SetRelativeLocation _destructible _fall false true)
      (Transformation|SetRelativeScale3D _destructible _scaleanim))))

(event Collision|EventActorBeginOverlap
  (params (OtherActor :type Actor%20Object%20Reference)))

(event EventTick
  (params (DeltaSeconds :type Float%20%28single-precision%29)))

(fn ConstructionScript)